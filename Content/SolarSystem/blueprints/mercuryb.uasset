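; Mercury actor for a solar system scene, scripted to circle the world origin in the XY plane.
; Each Tick adds delta time to Translate and sets the location from the sine and cosine of that time scaled by Velocity, times Distance.
; The angle is divided by a literal zero, which Blueprint evaluates as zero, so as written the planet stays fixed at Distance along Y.
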(event EventTick
  (params (DeltaSeconds :type Float%20%28single-precision%29))
  (bind _distance (Variables|Default|GetDistance))
  (Utilities|FlowControl|Sequence
    (:then_1
      (bind _output_get (Variables|Default|SetTranslate (+ DeltaSeconds (Variables|Default|GetTranslate))))
      (Transformation|SetActorLocation (Math|Vector|MakeVector (* (Math|Trig|Sin(Radians) (/ (* _output_get (Variables|Default|GetVelocity)) 0.0)) _distance) (* (Math|Trig|Cos(Radians) (/ (* _output_get (Variables|Default|GetVelocity)) 0.0)) _distance) 0.0) false false))))

(fn ConstructionScript)